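; Hit reaction component for BP_ThirdPersonCharacter that plays a directional hit montage when HitReact fires with an instigator.
; It computes a signed angle between the instigator-to-owner vector and the owner's forward vector via dot and cross products, printing it for debug.
; The angle maps to 90-degree front, back, left or right sectors, selecting the montage played on the owner's mesh after the parent HitReact runs.
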(event EventBeginPlay
  (bind _asbp_third_person_character (Utilities|Casting|CastToBP_ThirdPersonCharacter (Components|GetOwner)))
  (Variables|Default|SetOwnerRef _asbp_third_person_character))

(event EventTick
  (params (DeltaSeconds :type Float%20%28single-precision%29)))

(event EventHitReact
  (params (Instigator :type TGD%20Nekki%20Character%20Object%20Reference))
  (|CallParentFunction 0)
  (bind _resultangle (CallFunction|FindAngleBetweenActors Instigator))
  (bind _newparam (CallFunction|GetDirection _resultangle))
  (Animation|Montage|PlayMontage (Variables|/Script/Engine.Character|GetMesh (Variables|Default|GetOwnerRef)) (Utilities|Select :Index _newparam :NewEnumerator0 "/Game/Nekki/Assets/Character/Animations/Converted/HitReact/AM_HitReact_Front.AM_HitReact_Front" :NewEnumerator1 "/Game/Nekki/Assets/Character/Animations/Converted/HitReact/AM_HitReact_Back.AM_HitReact_Back" :NewEnumerator2 "/Game/Nekki/Assets/Character/Animations/Converted/HitReact/AM_HitReact_Left.AM_HitReact_Left" :NewEnumerator3 "/Game/Nekki/Assets/Character/Animations/Converted/HitReact/AM_HitReactRight.AM_HitReactRight")))

(fn FindAngleBetweenActors
  (params (Instigator :type TGD%20Nekki%20Character%20Object%20Reference))
  (bind _ownerref (Variables|Default|GetOwnerRef))
  (bind _ownerref_2 (Variables|Default|GetOwnerRef))
  (bind _returnvalue (Transformation|GetActorLocation Instigator))
  (bind _returnvalue_2 (Transformation|GetActorLocation _ownerref_2))
  (bind _returnvalue_3 (Transformation|GetActorForwardVector _ownerref))
  (bind _returnvalue_4 (- _returnvalue_2 _returnvalue))
  (bind _returnvalue_5 (Math|Vector|Normalize _returnvalue_4))
  (bind _returnvalue_6 (Math|Vector|DotProduct _returnvalue_5 _returnvalue_3))
  (bind _returnvalue_7 (Class|KismetMathLibrary|DegAcos _returnvalue_6))
  (bind _output_get (LocalVariables|SetAngle (Math|Float|SelectFloat _returnvalue_7 (* _returnvalue_7 -1.0) (< (.z (Math|Vector|CrossProduct _returnvalue_5 _returnvalue_3)) 0.0))))
  (Development|PrintString (Utilities|String|ToString(Float) _output_get))
  (return (LocalVariables|GetAngle)))

(fn GetDirection
  (params (Angle :type Float%20%28double-precision%29))
  (bind _returnvalue (Math|Float|Absolute(Float) Angle))
  (bind _returnvalue_2 (Math|Float|Absolute(Float) Angle))
  (if (and (>= _returnvalue_2 0.0) (<= _returnvalue_2 45.0))
    (return "NewEnumerator0")
    (elif (and (>= _returnvalue 135.0) (<= _returnvalue 1.8e+02))
      (return "NewEnumerator1")
      (elif (> Angle 0.0)
        (return "NewEnumerator3")
        (else
          (return "NewEnumerator2"))))))