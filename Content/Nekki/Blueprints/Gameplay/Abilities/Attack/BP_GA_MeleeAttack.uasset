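; Melee attack gameplay ability that snaps the character toward an enemy and plays the current combo montage.
; It sphere-traces nearby pawns, takes the first after sorting by angle, and lunges to it with root motion move-to force.
; The montage's "Hit" notify applies the damage GameplayEffect to that target.
; The ability registers itself with the FightingComponent, and StartNextAttack ends it and asks that component to activate the next attack.
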(event Ability|EventActivateAbility
  (bind _targetenemy (Variables|Default|GetTargetEnemy))
  (bind _returnvalue (Transformation|GetActorLocation _targetenemy))
  (bind _asbp_third_person_character (Utilities|Casting|CastToBP_ThirdPersonCharacter (Ability|GetAvatarActorfromActorInfo)))
  (Variables|Default|SetCharRef _asbp_third_person_character)
  (CallFunction|FindNearestEnemy)
  ;[1 1 1] Temp solution, need to create ability task further
  (Transformation|SetActorRotation (Variables|Default|GetCharRef) (Math|Rotator|FindLookatRotation (Transformation|GetActorLocation (Variables|Default|GetCharRef)) _returnvalue))
  (Ability|Tasks|ApplyRootMotionMoveToForce "None" _returnvalue 0.2 false "MOVE_None" false 0 "MaintainLastRootMotionVelocity"
    (:then
      (Variables|/Script/TGD_Nekki.FightingComponent|SetCurrentAttackAbility (Variables|/Script/TGD_Nekki.TGD_NekkiCharacter|GetFightingComponent (Variables|Default|GetCharRef)) self)
      (bind _notifyname (Animation|Montage|PlayMontage (Variables|/Script/Engine.Character|GetMesh (Variables|Default|GetCharRef)) (Variables|/Script/TGD_Nekki.MeleeAttackDataAsset|GetMontage (Utilities|Array|Get(acopy) (Variables|/Script/TGD_Nekki.FightingComponent|GetComboQueue (Variables|/Script/TGD_Nekki.TGD_NekkiCharacter|GetFightingComponent (Variables|Default|GetCharRef))) (Variables|/Script/TGD_Nekki.FightingComponent|GetCurrentMeleeAttackDataIndex (Variables|/Script/TGD_Nekki.TGD_NekkiCharacter|GetFightingComponent (Variables|Default|GetCharRef))))))
        (:OnCompleted
          (Ability|EndAbility))
        (:OnNotifyBegin
          (if (== _notifyname "Hit")
            (GameplayEffects|ApplyGameplayEffectToTarget (Ability|GetAbilitySystemComponent (Variables|Default|GetCharRef)) "/Game/Nekki/Blueprints/Gameplay/Effects/BP_GE_Damage.BP_GE_Damage_C" (Ability|GetAbilitySystemComponent (Variables|Default|GetTargetEnemy)) 1.0 (Utilities|Struct|MakeGameplayEffectContextHandle))))))))

(event Ability|EventOnEndAbility
  (params (bWasCancelled :type Boolean))
  (bind _charref (Variables|Default|GetCharRef)
    (:then
      (Variables|/Script/TGD_Nekki.FightingComponent|SetCurrentAttackAbility (Variables|/Script/TGD_Nekki.TGD_NekkiCharacter|GetFightingComponent _charref) 0))
    (:else)))

(event EventStartNextAttack
  (Ability|EndAbility)
  (bind _charref (Variables|Default|GetCharRef)
    (:then
      (Class|FightingComponent|ActivateCurrentAttackAbility (Variables|/Script/TGD_Nekki.TGD_NekkiCharacter|GetFightingComponent _charref)))
    (:else)))

(fn FindNearestEnemy
  (bind _charref (Variables|Default|GetCharRef))
  (bind _returnvalue (Transformation|GetActorLocation _charref))
  (bind _outhits (Collision|MultiSphereTraceForObjects _returnvalue _returnvalue 6e+02 (Utilities|Array|MakeArray "ObjectTypeQuery3") false (Utilities|Array|MakeArray (Variables|Default|GetCharRef)) "ForDuration"))
  (for _array_element _outhits
    (Utilities|Array|AddUnique (LocalVariables|GetActorsInSphere) (.HitActor (Collision|BreakHitResult _array_element))))
  (bind _returnvalue_2 (Class|AttackGameplayAbility|SortArraybyAngle (Variables|Default|GetCharRef) (LocalVariables|GetActorsInSphere)))
  (bind _output_get (LocalVariables|SetActorsInSphere _returnvalue_2))
  (Variables|Default|SetTargetEnemy (Utilities|Array|Get(acopy) _output_get)))