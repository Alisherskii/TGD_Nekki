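; Melee attack gameplay ability that lunges the character at a nearby pawn and plays the current combo montage.
; A 600-unit sphere trace gathers pawns, sorts them by angle and targets the first, then a short root-motion move drives toward it.
; The montage comes from the FightingComponent's ComboQueue, and the ability registers itself there while active.
; StartNextAttack ends this ability and has the component activate the next attack, chaining combos.
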(event Ability|EventActivateAbility
  (bind _asbp_third_person_character (Utilities|Casting|CastToBP_ThirdPersonCharacter (Ability|GetAvatarActorfromActorInfo)))
  (Variables|Default|SetCharRef _asbp_third_person_character)
  (CallFunction|FindNearestEnemy)
  (Ability|Tasks|ApplyRootMotionMoveToForce "None" (Transformation|GetActorLocation (Variables|Default|GetTargetEnemy)) 0.2 false "MOVE_None" false 0 "MaintainLastRootMotionVelocity"
    (:then
      (Variables|/Script/TGD_Nekki.FightingComponent|SetCurrentAttackAbility (Variables|/Script/TGD_Nekki.TGD_NekkiCharacter|GetFightingComponent (Variables|Default|GetCharRef)) self)
      (Animation|Montage|PlayMontage (Variables|/Script/Engine.Character|GetMesh (Variables|Default|GetCharRef)) (Variables|/Script/TGD_Nekki.MeleeAttackDataAsset|GetMontage (Utilities|Array|Get(acopy) (Variables|/Script/TGD_Nekki.FightingComponent|GetComboQueue (Variables|/Script/TGD_Nekki.TGD_NekkiCharacter|GetFightingComponent (Variables|Default|GetCharRef))) (Variables|/Script/TGD_Nekki.FightingComponent|GetCurrentMeleeAttackDataIndex (Variables|/Script/TGD_Nekki.TGD_NekkiCharacter|GetFightingComponent (Variables|Default|GetCharRef)))))
        (:OnCompleted
          (Ability|EndAbility))))))

(event Ability|EventOnEndAbility
  (params (bWasCancelled :type Boolean))
  (bind _charref (Variables|Default|GetCharRef)
    (:then
      (Variables|/Script/TGD_Nekki.FightingComponent|SetCurrentAttackAbility (Variables|/Script/TGD_Nekki.TGD_NekkiCharacter|GetFightingComponent _charref) 0))
    (:else)))

(event EventStartNextAttack
  (Ability|EndAbility)
  (bind _charref (Variables|Default|GetCharRef)
    (:then
      (Class|FightingComponent|ActivateCurrentAttackAbility (Variables|/Script/TGD_Nekki.TGD_NekkiCharacter|GetFightingComponent _charref)))
    (:else)))

(fn FindNearestEnemy
  (bind _charref (Variables|Default|GetCharRef))
  (bind _returnvalue (Transformation|GetActorLocation _charref))
  (bind _outhits (Collision|MultiSphereTraceForObjects _returnvalue _returnvalue 6e+02 (Utilities|Array|MakeArray "ObjectTypeQuery3") false (Utilities|Array|MakeArray (Variables|Default|GetCharRef)) "ForDuration"))
  (for _array_element _outhits
    (Utilities|Array|AddUnique (LocalVariables|GetActorsInSphere) (.HitActor (Collision|BreakHitResult _array_element))))
  (bind _returnvalue_2 (Class|AttackGameplayAbility|SortArraybyAngle (Variables|Default|GetCharRef) (LocalVariables|GetActorsInSphere)))
  (bind _output_get (LocalVariables|SetActorsInSphere _returnvalue_2))
  (Variables|Default|SetTargetEnemy (Utilities|Array|Get(acopy) _output_get)))