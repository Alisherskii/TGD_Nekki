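; BP_Destructible is a breakable prop that shatters when a pushed-back doll character slams into it.
; On a Box hit, it checks the character's ability system for the pushed-back gameplay tag, then destroys the Box and spawns FS_Damage at the impact point.
; When the chamfer cube Geometry Collection reports a Chaos break, the actor waits for Lifetime and destroys itself.
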(event OnComponentHit(Box)
  (params (HitComponent :type Primitive%20Component%20Object%20Reference) (OtherActor :type Actor%20Object%20Reference) (OtherComp :type Primitive%20Component%20Object%20Reference) (NormalImpulse :type Vector :default "0, 0, 0") (Hit :type Hit%20Result%20Structure%20%28by%20ref%29))
  (bind _asbp_third_person_character_doll (Utilities|Casting|CastToBP_ThirdPersonCharacter_Doll OtherActor))
  (if (GameplayTags|HasMatchingGameplayTag (Ability|GetAbilitySystemComponent _asbp_third_person_character_doll) "(TagName=\"State.Negativbe.PushedBack\")")
    (Components|DestroyComponent (Variables|Default|GetBox))
    (Game|SpawnActorfromClass "/Game/Nekki/Blueprints/Gameplay/Effects/FS_Damage.FS_Damage_C" (Math|Transform|MakeTransform (.Location (Collision|BreakHitResult Hit)) "0, 0, 0" "1.000000,1.000000,1.000000") "Undefined" "MultiplyWithRoot" 0 0)))

(event OnChaosBreakEvent(SM_ChamferCube_GeometryCollection)
  (params (BreakEvent :type Chaos%20Break%20Event%20Structure%20%28by%20ref%29))
  (Utilities|FlowControl|Delay (Variables|Default|GetLifetime))
  (Actor|DestroyActor))

(event EventBeginPlay)

(event Collision|EventActorBeginOverlap
  (params (OtherActor :type Actor%20Object%20Reference)))

(event EventTick
  (params (DeltaSeconds :type Float%20%28single-precision%29)))

(fn ConstructionScript)